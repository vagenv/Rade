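; Rifle weapon Blueprint that handles the animation side of firing, alt-firing and reloading.
; Fire, AltFire and ReloadStart each forward to a matching Global event call.
; The Global fire, alt-fire and reload event handlers play single-fire, double-fire and reload animations once on both the first-person and third-person meshes.
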(event `self.ReceiveBeginPlay`)

(event `self.ReceiveTick`
  (params (DeltaSeconds :type "Float (single-precision)")))

(event `self.BP_Fire`
  (`self.Global_Fire_Event`))

(event `self.BP_AltFire`
  (`self.Global_AltFire_Event`))

(event `self.BP_Reload_Start`
  (`self.Global_Reload_Event`))

(event `Global_Fire_Event`
  (`SkeletalMeshComponent.PlayAnimation` (`self.Mesh1P`) "/Game/Rade/Meshes/Weapons/AR/AR_SingleFire_Anim.AR_SingleFire_Anim" false)
  (`SkeletalMeshComponent.PlayAnimation` (`self.Mesh3P`) "/Game/Rade/Meshes/Weapons/AR/AR_SingleFire_Anim.AR_SingleFire_Anim" false))

(event `Global_AltFire_Event`
  (`SkeletalMeshComponent.PlayAnimation` (`self.Mesh1P`) "/Game/Rade/Meshes/Weapons/AR/AR_DoubleFire_Anim.AR_DoubleFire_Anim" false)
  (`SkeletalMeshComponent.PlayAnimation` (`self.Mesh3P`) "/Game/Rade/Meshes/Weapons/AR/AR_DoubleFire_Anim.AR_DoubleFire_Anim" false))

(event `Global_Reload_Event`
  (`SkeletalMeshComponent.PlayAnimation` (`self.Mesh3P`) "/Game/Rade/Meshes/Weapons/AR/AR_Reload.AR_Reload" false)
  (`SkeletalMeshComponent.PlayAnimation` (`self.Mesh1P`) "/Game/Rade/Meshes/Weapons/AR/AR_Reload.AR_Reload" false))

(fn `UserConstructionScript`)